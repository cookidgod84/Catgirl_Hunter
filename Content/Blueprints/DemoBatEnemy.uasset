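; DemoBatEnemy is a demo flipbook bat enemy that dies when it touches the player.
; Player-class overlap sets Killed and plays the death flipbook once, then destroys only the render component when playback finishes, leaving the actor.
; Tick sets location from GetEnemyMovement, whose move-toward-player calculation appears unconnected to any output in this graph.
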(event `self.ReceiveBeginPlay`
  (`self.K2_SetActorRotation` (struct :`Yaw` 90.0)))

(event `self.ReceiveActorBeginOverlap`
  (params (OtherActor :type "Actor Object Reference"))
  (if (== (`GameplayStatics.GetObjectClass` OtherActor) (`GameplayStatics.GetObjectClass` (`GameplayStatics.GetPlayerCharacter` 0)))
    (`PaperFlipbookComponent.SetLooping` (`self.RenderComponent`) false)
    (`PaperFlipbookComponent.SetFlipbook` (`self.RenderComponent`) "/Game/Enemies/basic_enemy_sprites/demo_bat_die.demo_bat_die")
    (`KismetSystemLibrary.PrintString` "hit player")
    (set `self.killed` true)))

(event `self.ReceiveTick`
  (params (DeltaSeconds :type "Float (single-precision)"))
  (`self.K2_SetActorLocation` (`self.GetEnemyMovement` DeltaSeconds)))

(event `self.RenderComponent.OnFinishedPlaying`
  (if (`self.killed`)
    (`ActorComponent.K2_DestroyComponent` (`self.RenderComponent`))))

(fn `UserConstructionScript`)