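; Player controller that handles character movement and a cooldown-gated dodge through Enhanced Input.
; On BeginPlay it adds the movement mapping context; move input becomes a normalized world-space direction applied at half scale.
; Dodge input blocks movement during a short delay, then teleports the character along the last movement direction and re-enables dodging after a reset time.
; The dodge also prints a debug string.
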(event `self.ReceiveBeginPlay`
  (bind _returnvalue (subsystem `EnhancedInputLocalPlayerSubsystem`))
  (`/Engine/EditorBlueprintResources/StandardMacros.IsValid` _returnvalue
    (:`Is Valid`
      (`EnhancedInputSubsystemInterface.AddMappingContext` _returnvalue "/Game/Blueprints/CharacterMovement.CharacterMovement" 0 (struct)))))

(event `self.ReceiveTick`
  (params (DeltaSeconds :type "Float (single-precision)")))

(event `EnhancedInput|/Game/Blueprints/InputActions/IA_Move`
  (params (ActionValue :type "Vector2D Structure") (ElapsedSeconds :type "Float (double-precision)") (TriggeredSeconds :type "Float (double-precision)") (InputAction :type "InputAction Object Reference" :default "/Game/Blueprints/InputActions/IA_Move.IA_Move"))
  (:`Triggered`
    (`self.Move` ActionValue)))

(event `EnhancedInput|/Game/Blueprints/InputActions/IA_DodgeRoll`
  (params (ActionValue :type Boolean) (ElapsedSeconds :type "Float (double-precision)") (TriggeredSeconds :type "Float (double-precision)") (InputAction :type "InputAction Object Reference" :default "/Game/Blueprints/InputActions/IA_DodgeRoll.IA_DodgeRoll"))
  (:`Triggered`
    (if (`self.CanDodge`)
      (set `self.CanDodge` false)
      (set `self.IsDodging` true)
      (`KismetSystemLibrary.Delay` (`self.DodgeDelay`))
      (`self.Dodge`)
      (set `self.IsDodging` false)
      (`KismetSystemLibrary.Delay` (`self.DodgeResetTime`))
      (set `self.CanDodge` true))))

(fn `Dodge`
  (locals (dodge_delay :type "Float (double-precision)" :default 0.5))
  (bind _returnvalue (`GameplayStatics.GetPlayerCharacter` 0))
  (`KismetSystemLibrary.PrintString` "Hello")
  (`self.K2_TeleportTo` _returnvalue (+ (`self.K2_GetActorLocation` _returnvalue) (* (`self.CurrentDirection`) (`self.DodgeDistance`))) (`self.K2_GetActorRotation` _returnvalue)))

(fn `Move`
  (params (Direction :type "Vector2D Structure"))
  (locals (move_speed :type "Float (double-precision)" :default 0.5) (dodge_distance :type "Float (double-precision)"))
  (if (not (`self.IsDodging`))
    (bind _output_get (set `self.CurrentDirection` (`KismetMathLibrary.Normal` (`KismetMathLibrary.Conv_Vector2DToVector` Direction))))
    (`Pawn.AddMovementInput` (`GameplayStatics.GetPlayerPawn` 0) _output_get 0.5 false)))

(fn `UserConstructionScript`)