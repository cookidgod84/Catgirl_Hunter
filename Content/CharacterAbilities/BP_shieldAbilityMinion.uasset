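; Shield ability minion actor that blocks enemy projectiles and pushes enemies away on contact.
; Collision overlaps destroy BP_BaseEnemyProjectile actors, or call ShoveEnemy on BP_BaseEnemy actors with a computed shove vector.
; The vector points outward from the attach parent of the Parent reference, falling back to the player character if Parent is invalid, scaled by Shovedistance.
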(event `self.ReceiveTick`
  (params (DeltaSeconds :type "Float (single-precision)"))
  (`parent.ReceiveTick` DeltaSeconds))

(event `self.Collision.OnComponentBeginOverlap`
  (params (OverlappedComponent :type "PrimitiveComponent Object Reference") (OtherActor :type "Actor Object Reference") (OtherComp :type "PrimitiveComponent Object Reference") (OtherBodyIndex :type Integer) (bFromSweep :type Boolean) (SweepResult :type "HitResult Structure (by ref)"))
  (bind _asbp_base_enemy_projectile (cast `/Game/Enemies/BP_BaseEnemyProjectile` OtherActor)
    (:`then`
      (`self.K2_DestroyActor` _asbp_base_enemy_projectile))
    (:`CastFailed`
      (bind _asbp_base_enemy (cast `/Game/Enemies/BP_BaseEnemy` OtherActor))
      (bind _shovevector (`self.Calculate Shove Vector` (`self.K2_GetActorLocation` _asbp_base_enemy)))
      (`/Game/Enemies/BP_BaseEnemy.ShoveEnemy` _asbp_base_enemy _shovevector))))

(fn `Calculate Shove Vector`
  (params (EnemyLocation :type "Vector Structure"))
  (returns (ShoveVector :type "Vector Structure"))
  (locals (origin :type "Vector Structure"))
  (if (`KismetSystemLibrary.IsValid` (`self.parent`))
    (bind _output_get (set `local.origin` (`SceneComponent.K2_GetComponentLocation` (`SceneComponent.GetAttachParent` (`self.parent`)))))
    (else
      (set `local.origin` (`self.K2_GetActorLocation` (`GameplayStatics.GetPlayerCharacter` 0)))))
  (return (* (`KismetMathLibrary.Normal` (- EnemyLocation _output_get)) (`self.shovedistance`))))

(fn `UserConstructionScript`
  (`parent.UserConstructionScript`))