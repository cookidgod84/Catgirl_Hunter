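; Bomb ability projectile, a Paper2D flipbook actor that arcs to a destination, explodes and damages enemies.
; BeginPlay builds a spline from start, destination and arc height; Tick moves only the render component along it using a fuse-scaled counter, feeding local-space spline locations as world positions.
; When the counter reaches FuseTime, Explode swaps to the explosion flipbook and damages BP_BaseEnemy pawns via a debug-drawn sphere trace.
; A timer destroys the actor after the animation.
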(event `self.ReceiveBeginPlay`
  (`SplineComponent.SetSplinePoints` (`self.bombTrajectory`) (`self.` (`SceneComponent.K2_GetComponentLocation` (`self.RenderComponent`)) (`self.bombDestination`) (`self.arcHeight`)) "Local" true))

(event `ReceiveActorBeginOverlap_1`
  (params (OtherActor :type "Actor Object Reference")))

(event `self.ReceiveTick`
  (params (DeltaSeconds :type "Float (single-precision)"))
  (bind _output_get (set `self.splineTimeCounter` (+ (* (/ DeltaSeconds (`self.fuseTime`)) 10.0) (`self.splineTimeCounter`))))
  (`SceneComponent.K2_SetWorldLocation` (`self.RenderComponent`) (`SplineComponent.GetLocationAtTime` (`self.bombTrajectory`) (/ _output_get (`self.fuseTime`)) "Local" false) false false)
  (if (and (>= (`self.splineTimeCounter`) (`self.fuseTime`)) (not (`self.exploded`)))
    (`self.explode`)
    (`KismetSystemLibrary.K2_SetTimerDelegate` (delegate `DestroyBomb`) (`PaperFlipbookComponent.GetFlipbookLength` (`self.RenderComponent`)))))

(event `DestroyBomb`
  (`Actor.K2_DestroyActor`))

(fn `explode`
  (bind _returnvalue (`SceneComponent.K2_GetComponentLocation` (`self.RenderComponent`)))
  (`PaperFlipbookComponent.SetLooping` (`self.RenderComponent`) false)
  (`PaperFlipbookComponent.SetFlipbook` (`self.RenderComponent`) "/Game/CharacterAbilities/assets/bombassets/Bomb_Explosion.Bomb_Explosion")
  (set `self.exploded` true)
  (bind _outhits (`KismetSystemLibrary.SphereTraceMultiForObjects` :`Start` _returnvalue :`End` _returnvalue :`Radius` (`self.explosionRadius`) :`ObjectTypes` (`|MakeArray` "ObjectTypeQuery3" :!type "EObjectTypeQuery Enum") :`DrawDebugType` "ForDuration" :`DrawTime` 1.0))
  (for _array_element _outhits
    (bind _asbp_base_enemy (cast `/Game/Enemies/BP_BaseEnemy` (`.HitActor` (`GameplayStatics.BreakHitResult` _array_element))))
    (`/Game/Enemies/BP_BaseEnemy.TakeDamage` _asbp_base_enemy (`self.bombDamage`))))

(fn `UserConstructionScript`
  (`SceneComponent.K2_SetRelativeRotation` (`self.RenderComponent`) (struct :`Yaw` 90.0) false false))