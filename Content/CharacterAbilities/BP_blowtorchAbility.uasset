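; Blowtorch character ability that periodically fires a burning flame sector from the location of the component it is attached to.
; Each tick advances a firing timer, and when it triggers, a blowtorch projectile actor spawns with fixed burn damage, burn duration and flame length.
; A sweep helper gives each shot a random facing angle and a fixed quarter-circle sector, so the flame is not aimed.
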(event `self.ReceiveTick`
  (params (DeltaSeconds :type "Float (single-precision)"))
  (`parent.ReceiveTick` DeltaSeconds)
  (bind _spawnprojectile (`self.Increment Firing Timer` DeltaSeconds))
  (if _spawnprojectile
    (bind (_angle _sectorsize) (`self.makeBlowTorchSweep`))
    (`|SpawnActorFromClass` "/Game/CharacterAbilities/BP_blowtorchAbilityProjectile.BP_blowtorchAbilityProjectile_C" (`KismetMathLibrary.Conv_VectorToTransform` (`self.K2_GetComponentLocation` (`self.GetAttachParent`))) "Undefined" "MultiplyWithRoot" null 3 5.0 _angle _sectorsize 400.0 null)))

(fn `makeBlowTorchSweep`
  (returns (angle :type "Float (double-precision)") (sectorsize :type "Float (double-precision)"))
  (return (`KismetMathLibrary.RandomFloatInRange` 0.0 359.0) 90.0))