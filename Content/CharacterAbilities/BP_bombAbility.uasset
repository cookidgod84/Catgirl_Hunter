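; Bomb ability component that periodically launches bomb projectiles from its attach parent toward random destinations.
; Each Tick advances a firing timer and, when it triggers, spawns BP_BombAbilityProjectile with start and end locations.
; MakeBombDestination sets X and Y to the minimum range plus a randomly signed fraction of the maximum range, without adding the parent's position.
; Only the destination's Z comes from the parent.
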(event `self.ReceiveTick`
  (params (DeltaSeconds :type "Float (single-precision)"))
  (bind _spawnprojectile (`self.Increment Firing Timer` DeltaSeconds))
  (if _spawnprojectile
    (bind _bombtransform (`self.makeBombDestination`))
    (`|SpawnActorFromClass` "/Game/CharacterAbilities/BP_BombAbilityProjectile.BP_BombAbilityProjectile_C" (`KismetMathLibrary.Conv_VectorToTransform` (`self.K2_GetComponentLocation` (`self.GetAttachParent`))) "Undefined" "MultiplyWithRoot" null (`self.K2_GetComponentLocation` (`self.GetAttachParent`)) _bombtransform 0.0 null)))

(fn `makeBombDestination`
  (returns (bombTransform :type "Vector Structure"))
  (locals (negators :type "Array of Integer"))
  (return (`KismetMathLibrary.MakeVector` (+ (`self.minBombRange`) (* (* (`self.maxBombRange`) (`KismetMathLibrary.RandomFloat`)) (`|GetArrayItem` (`local.negators`) (`KismetMathLibrary.Conv_Int64ToInt` (`KismetMathLibrary.RandomInteger64InRange` 0 1))))) (+ (`self.minBombRange`) (* (* (`self.maxBombRange`) (`KismetMathLibrary.RandomFloat`)) (`|GetArrayItem` (`local.negators`) (`KismetMathLibrary.Conv_Int64ToInt` (`KismetMathLibrary.RandomInteger64InRange` 0 1))))) (.z (`self.K2_GetComponentLocation` (`self.GetAttachParent`))))))