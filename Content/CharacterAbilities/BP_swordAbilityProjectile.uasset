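; BP_swordAbilityProjectile is the projectile actor for a sword ability, damaging enemies it overlaps.
; On BeginPlay it sets its life span from Lifespan, and HitCollider overlaps that pass IsValidEnemy apply Damage through BP_BaseEnemy's TakeDamage.
; It is not destroyed on hit, and no movement logic appears in its graphs.
; The construction script sets a fixed 90-degree rotation and zeroes its relative location.
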(event `self.ReceiveBeginPlay`
  (`self.SetLifeSpan` (`self.lifespan`)))

(event `self.hit collider.OnComponentBeginOverlap`
  (params (OverlappedComponent :type "PrimitiveComponent Object Reference") (OtherActor :type "Actor Object Reference") (OtherComp :type "PrimitiveComponent Object Reference") (OtherBodyIndex :type Integer) (bFromSweep :type Boolean) (SweepResult :type "HitResult Structure (by ref)"))
  (if (`/Game/CharacterAbilities/BML_characterAbilityMacros.isValidEnemy` OtherActor)
    (bind _asbp_base_enemy (cast `/Game/Enemies/BP_BaseEnemy` OtherActor))
    (`/Game/Enemies/BP_BaseEnemy.TakeDamage` _asbp_base_enemy (`self.damage`))))

(fn `UserConstructionScript`
  (`self.K2_SetActorRotation` (struct :`Roll` 90.0))
  (`self.K2_SetActorRelativeLocation` (0.0 0.0 0.0)))