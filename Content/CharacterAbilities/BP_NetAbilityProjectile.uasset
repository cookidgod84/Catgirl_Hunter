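; Thrown-net ability projectile that stuns enemies in an area on impact.
; Each tick it sweeps the net's collision along the Trajectory spline by normalized time, destroying itself at the end if nothing is hit.
; On overlapping a valid enemy it stops, sphere-traces one radius ahead along the spline direction and stuns every BP_BaseEnemy found for the netted duration.
; The net flipbook then stops looping, and the actor is destroyed when it finishes playing.
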(event `self.ReceiveTick`
  (params (DeltaSeconds :type "Float (single-precision)"))
  (`parent.ReceiveTick` DeltaSeconds)
  (if (not (`self.HitEnemy`))
    (set `self.CurrentTimeOnSpline` (+ (/ (* DeltaSeconds 1000.0) (`self.TimeToTravelSpline`)) (`self.CurrentTimeOnSpline`)))
    (if (< (`self.CurrentTimeOnSpline`) 1.0)
      (`SceneComponent.K2_SetWorldLocation` (`self.NetCollision`) (`SplineComponent.GetLocationAtTime` (`self.Trajectory`) (`self.CurrentTimeOnSpline`) "Local" false) true false)
      (else
        (`self.K2_DestroyActor`)))))

(event `self.NetCollision.OnComponentBeginOverlap`
  (params (OverlappedComponent :type "PrimitiveComponent Object Reference") (OtherActor :type "Actor Object Reference") (OtherComp :type "PrimitiveComponent Object Reference") (OtherBodyIndex :type Integer) (bFromSweep :type Boolean) (SweepResult :type "HitResult Structure (by ref)"))
  (bind _returnvalue (+ (* (`SplineComponent.GetDirectionAtTime` (`self.Trajectory`) (`self.CurrentTimeOnSpline`) "Local" false) (`self.NetRadius`)) (`SceneComponent.K2_GetComponentLocation` (`self.NetCollision`))))
  (if (`/Game/CharacterAbilities/GenericClasses/BML_characterAbilityMacros.isValidEnemy` OtherActor)
    (set `self.HitEnemy` true)
    (`PaperFlipbookComponent.SetLooping` (`self.NetFlipbook`) false)
    (bind _outhits (`KismetSystemLibrary.SphereTraceMultiForObjects` _returnvalue _returnvalue (`self.NetRadius`) (`|MakeArray` "ObjectTypeQuery3" :!type "EObjectTypeQuery Enum")))
    (for _array_element _outhits
      (bind _asbp_base_enemy (cast `/Game/Enemies/BP_BaseEnemy` (`.HitActor` (`GameplayStatics.BreakHitResult` _array_element))))
      (`/Game/Enemies/BP_BaseEnemy.StunEnemy` _asbp_base_enemy (`self.NettedDuration`)))))

(event `self.NetFlipbook.OnFinishedPlaying`
  (`self.K2_DestroyActor`))

(fn `UserConstructionScript`
  (`parent.UserConstructionScript`)
  (`SceneComponent.K2_SetRelativeRotation` (`self.NetFlipbook`) (struct :`Yaw` 90.0) false false))