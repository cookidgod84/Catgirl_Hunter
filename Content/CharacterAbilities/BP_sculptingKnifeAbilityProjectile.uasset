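; Homing knife projectile for the sculpting knife ability that damages enemies it overlaps.
; Each tick it accelerates toward its target with velocity damping and a speed cap, moving by swept location updates.
; Hitting the target triggers a shuffled sphere trace around the player for another enemy and briefly disables collision.
; Without a valid target it retries the search; debug spheres and prints remain active.
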(event `FindTarget`
  (`self.findNextTarget`)
  (if (not (`KismetSystemLibrary.IsValid` (`self.target`)))
    (`KismetSystemLibrary.K2_SetTimerDelegate` (delegate `FindTarget`) 0.5)))

(event `self.ReceiveBeginPlay`
  (`parent.ReceiveBeginPlay`))

(event `ResetCollisions`
  (`PrimitiveComponent.SetCollisionEnabled` (`self.collision`) "NoCollision")
  (`KismetSystemLibrary.K2_SetTimerDelegate` (delegate `EnableCollision`) 0.5))

(event `EnableCollision`
  (`PrimitiveComponent.SetCollisionEnabled` (`self.collision`) "QueryAndPhysics"))

(event `self.ReceiveTick`
  (params (DeltaSeconds :type "Float (single-precision)"))
  (`parent.ReceiveTick` DeltaSeconds)
  (if (`KismetSystemLibrary.IsValid` (`self.target`))
    (`self.accelerateKnife` DeltaSeconds)
    (`self.K2_SetActorLocation` (+ (`self.K2_GetActorLocation`) (`self.knifespeedvector`)) true)
    (`KismetSystemLibrary.DrawDebugSphere` (`self.K2_GetActorLocation` (`self.target`)) 100.0 12 (struct :`R` 1.0 :`G` 1.0 :`B` 1.0 :`A` 1.0) 0.1 1.0)
    (else
      (`self.FindTarget`))))

(event `self.collision.OnComponentBeginOverlap`
  (params (OverlappedComponent :type "PrimitiveComponent Object Reference") (OtherActor :type "Actor Object Reference") (OtherComp :type "PrimitiveComponent Object Reference") (OtherBodyIndex :type Integer) (bFromSweep :type Boolean) (SweepResult :type "HitResult Structure (by ref)"))
  (bind _asbp_base_enemy (cast `/Game/Enemies/BP_BaseEnemy` OtherActor))
  (`/Game/Enemies/BP_BaseEnemy.TakeDamage` _asbp_base_enemy (`self.damage`))
  (if (== _asbp_base_enemy (`self.target`))
    (`self.findNextTarget`)
    (`KismetSystemLibrary.PrintString` "getting new target")
    (else
      (`KismetSystemLibrary.PrintString` "hit enemy"))))

(fn `accelerateKnife`
  (params (deltaTime :type "Float (double-precision)"))
  (bind _knifemaxspeed (`self.knifemaxspeed`))
  (set `self.knifespeedvector` (`KismetMathLibrary.ClampVectorSize` (+ (* (`KismetMathLibrary.Normal` (- (`self.K2_GetActorLocation` (`self.target`)) (`self.K2_GetActorLocation`))) (`self.knifeacceleration`) deltaTime) (* (`self.knifespeedvector`) 0.95)) (* _knifemaxspeed -1.0) _knifemaxspeed)))

(fn `findNextTarget`
  (bind _returnvalue (`self.K2_GetActorLocation` (`GameplayStatics.GetPlayerPawn` 0)))
  (bind _outhits (`KismetSystemLibrary.SphereTraceMultiForObjects` _returnvalue _returnvalue (`self.newtargetsearchradius`) (`|MakeArray` "ObjectTypeQuery3" :!type "EObjectTypeQuery Enum") false (`|MakeArray` (`self.target`) :!type "Actor Object Reference") "ForDuration" true (struct :`R` 1.0 :`A` 1.0) (struct :`G` 1.0 :`A` 1.0) 1.0))
  (`KismetArrayLibrary.Array_Shuffle` _outhits)
  (for _array_element _outhits
    (bind _asbp_base_enemy (cast `/Game/Enemies/BP_BaseEnemy` (`.HitActor` (`GameplayStatics.BreakHitResult` _array_element))))
    (set `self.target` _asbp_base_enemy)
    (break))
  (`self.ResetCollisions`))

(fn `UserConstructionScript`
  (`parent.UserConstructionScript`))