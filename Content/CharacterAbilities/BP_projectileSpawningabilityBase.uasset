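; Base scene component for projectile-spawning character abilities, providing fire-rate timing and nearest-enemy targeting helpers.
; IncrementFiringTimer accumulates delta time and returns true when the fire rate interval elapses, carrying the overshoot forward.
; FindNearestEnemyLocation scans supplied enemies from the attach parent, returning the tracked nearest enemy's location or the parent's if invalid.
; The event graph is empty and the nearest-distance variable is never reset here.
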(fn `findNearestEnemyLocation`
  (params (Enemies :type "Array of /Game/Enemies/BP_BaseEnemy Object Reference"))
  (returns (nearestEnemyLocation :type "Vector Structure"))
  (locals (nearestEnemyDistance :type "Float (double-precision)" :default 1000000.0) (currentNearestEnemy :type "/Game/Enemies/BP_BaseEnemy Object Reference"))
  (for _array_element Enemies
    (bind _returnvalue (`KismetMathLibrary.Vector_Distance` (`Actor.K2_GetActorLocation` _array_element) (`self.K2_GetComponentLocation` (`self.GetAttachParent`))))
    (if (< _returnvalue (`local.nearestEnemyDistance`))
      (set `local.nearestEnemyDistance` _returnvalue)
      (set `local.currentNearestEnemy` _array_element)))
  (if (`KismetSystemLibrary.IsValid` (`local.currentNearestEnemy`))
    (return (`Actor.K2_GetActorLocation` (`local.currentNearestEnemy`)))
    (else
      (return (`self.K2_GetComponentLocation` (`self.GetAttachParent`))))))

(fn `Increment Firing Timer`
  (params (deltaTime :type "Float (double-precision)"))
  (returns (spawnProjectile :type Boolean))
  (bind _output_get (set `self.fireRateCounter` (+ deltaTime (`self.fireRateCounter`))))
  (if (>= _output_get (`self.fireRate`))
    (set `self.fireRateCounter` (- (`self.fireRateCounter`) (`self.fireRate`)))
    (return true)
    (else
      (return false))))