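; Whip ability projectile that visually strikes from a start point to an end point, damaging a target enemy and slowing nearby enemies.
; A non-looping flipbook is rotated and stretched by sprite width to span the two points.
; When it finishes, it hides, triggers the shockwave, and damages the target if still near the endpoint.
; A short timer then sphere-traces pawns to slow enemies, and the actor destroys itself when the shockwave effect ends.
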(event `self.ReceiveBeginPlay`
  (bind _returnvalue (- (`self.endlocation`) (`self.startlocation`)))
  (`parent.ReceiveBeginPlay`)
  (`PaperFlipbookComponent.SetLooping` (`self.WhipFlipbook`) false)
  (`SceneComponent.K2_SetWorldRotation` (`self.WhipFlipbook`) (`KismetMathLibrary.MakeRotationFromAxes` _returnvalue (0.0 1.0 0.0)) false false)
  (`SceneComponent.SetWorldScale3D` (`self.WhipFlipbook`) (`KismetMathLibrary.MakeVector` (/ (`KismetMathLibrary.VSize` _returnvalue) (`KismetMathLibrary.BreakVector2D` (`MyPaper2DFunctions.GetSourceSize` (`PaperFlipbook.GetSpriteAtFrame` (`PaperFlipbookComponent.GetFlipbook` (`self.WhipFlipbook`)) 0)))) 1.0 0.2))
  (`SceneComponent.K2_SetWorldLocation` (`self.Shockwave`) (`KismetMathLibrary.MakeVector` (.x (`self.endlocation`)) (.y (`self.endlocation`))) false false))

(event `SlowFromShockwave`
  (bind _outhits (`KismetSystemLibrary.SphereTraceMultiForObjects` (`self.endlocation`) (`self.endlocation`) (`self.shockwaveradius`) (`|MakeArray` "ObjectTypeQuery3" :!type "EObjectTypeQuery Enum") false (`|MakeArray` (`GameplayStatics.GetPlayerCharacter` 0))))
  (for _array_element _outhits
    (bind _asbp_base_enemy (cast `/Game/Enemies/BP_BaseEnemy` (`.HitActor` (`GameplayStatics.BreakHitResult` _array_element))))
    (`/Game/Enemies/BP_BaseEnemy.SlowEnemy` _asbp_base_enemy 0.5 1.0)))

(event `self.WhipFlipbook.OnFinishedPlaying`
  (`SceneComponent.SetVisibility` (`self.WhipFlipbook`) false false)
  (`ActorComponent.Activate` (`self.Shockwave`) false)
  (if (`KismetSystemLibrary.IsValid` (`self.targetenemy`))
    (if (< (`KismetMathLibrary.Vector_Distance` (`self.K2_GetActorLocation` (`self.targetenemy`)) (`self.endlocation`)) (`self.hitdistance`))
      (`/Game/Enemies/BP_BaseEnemy.TakeDamage` (`self.targetenemy`) (`self.damage`))))
  (`KismetSystemLibrary.K2_SetTimerDelegate` (delegate `SlowFromShockwave`) 0.2))

(event `self.Shockwave.OnSystemFinished`
  (params (PSystem :type "NiagaraComponent Object Reference"))
  (`self.K2_DestroyActor`))

(fn `UserConstructionScript`)