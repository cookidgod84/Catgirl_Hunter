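; BP_chiselProjectile is a thrown chisel ability projectile that damages enemies deriving from BP_BaseEnemy.
; Construction sets a base mesh-style orientation on the actor, and BeginPlay yaws it to the heading of Direction and starts a Lifespan self-destruct timer.
; Tick moves it along Direction at Speed with a swept offset.
; Overlapping an enemy applies Damage and schedules destruction after a short delay, during which it keeps moving.
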(event `self.collision.OnComponentBeginOverlap`
  (params (OverlappedComponent :type "PrimitiveComponent Object Reference") (OtherActor :type "Actor Object Reference") (OtherComp :type "PrimitiveComponent Object Reference") (OtherBodyIndex :type Integer) (bFromSweep :type Boolean) (SweepResult :type "HitResult Structure (by ref)"))
  (bind _asbp_base_enemy (cast `/Game/Enemies/BP_BaseEnemy` OtherActor))
  (`/Game/Enemies/BP_BaseEnemy.TakeDamage` _asbp_base_enemy (`self.damage`))
  (`KismetSystemLibrary.K2_SetTimerDelegate` (delegate `DestroyChisel`) 0.25))

(event `DestroyChisel`
  (`self.K2_DestroyActor`))

(event `self.ReceiveBeginPlay`
  (`parent.ReceiveBeginPlay`)
  (`KismetSystemLibrary.K2_SetTimerDelegate` (delegate `DestroyChisel`) (`self.lifespan`))
  (`self.K2_AddActorWorldRotation` (`KismetMathLibrary.RotatorFromAxisAndAngle` (0.0 0.0 1.0) (`KismetMathLibrary.RadiansToDegrees` (`KismetMathLibrary.Vector_HeadingAngle` (`self.direction`))))))

(event `self.ReceiveTick`
  (params (DeltaSeconds :type "Float (single-precision)"))
  (`parent.ReceiveTick` DeltaSeconds)
  (`self.K2_AddActorWorldOffset` (* (`self.direction`) DeltaSeconds (`self.speed`)) true))

(fn `UserConstructionScript`
  (`parent.UserConstructionScript`)
  (`self.K2_SetActorRotation` (struct :`Yaw` 225.0 :`Roll` 90.0)))