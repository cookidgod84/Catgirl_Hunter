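; Shield ability component that surrounds its attach parent with orbiting BP_shieldAbilityMinion actors, starting with three on BeginPlay.
; AddShield spawns a minion, stores it in Shields and respaces all shields evenly, placing them with the parent's forward vector as axis.
; Each tick, SpinShields advances every shield's stored angle and sweeps it to a position at the rotation radius, using the parent's up vector as axis.
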(event `self.ReceiveBeginPlay`
  (`parent.ReceiveBeginPlay`)
  (`self.addShield`)
  (`self.addShield`)
  (`self.addShield`))

(event `self.ReceiveTick`
  (params (DeltaSeconds :type "Float (single-precision)"))
  (`parent.ReceiveTick` DeltaSeconds)
  (`self.spinShields` DeltaSeconds))

(fn `addShield`
  (bind _shields (`self.shields`))
  (bind _returnvalue (`|SpawnActorFromClass` "/Game/CharacterAbilities/BP_shieldAbilityMinion.BP_shieldAbilityMinion_C" (`self.K2_GetComponentToWorld` (`self.GetAttachParent`)) "Undefined" "MultiplyWithRoot" null self null))
  (`KismetArrayLibrary.Array_Add` (`self.shields`) _returnvalue)
  ;[1 1 1] evenly space the new number of shields
  (for (_array_element _array_index) _shields
    (bind _returnvalue_2 (* (/ _array_index (`KismetArrayLibrary.Array_Length` _shields)) 360.0))
    (set `/Game/CharacterAbilities/BP_shieldAbilityMinion.currentrotation` _returnvalue_2 _array_element)
    (bind _returnvalue_3 (`KismetMathLibrary.RotatorFromAxisAndAngle` (`self.GetForwardVector` (`self.GetAttachParent`)) _returnvalue_2))
    (`Actor.K2_SetActorLocationAndRotation` _array_element (+ (* (`KismetMathLibrary.GetForwardVector` _returnvalue_3) (`self.rotationradius`)) (`self.K2_GetComponentLocation` (`self.GetAttachParent`))) _returnvalue_3 true false)))

(fn `spinShields`
  (params (`Delta Seconds` :type "Float (double-precision)"))
  (for _array_element (`self.shields`)
    (bind _returnvalue (+ (`/Game/CharacterAbilities/BP_shieldAbilityMinion.currentrotation` _array_element) (* (`self.rotationspeed`) `Delta Seconds`)))
    (set `/Game/CharacterAbilities/BP_shieldAbilityMinion.currentrotation` _returnvalue _array_element)
    (bind _returnvalue_2 (`KismetMathLibrary.RotatorFromAxisAndAngle` (`self.GetUpVector` (`self.GetAttachParent`)) _returnvalue))
    (`Actor.K2_SetActorLocationAndRotation` _array_element (+ (* (`KismetMathLibrary.GetForwardVector` _returnvalue_2) (`self.rotationradius`)) (`self.K2_GetComponentLocation` (`self.GetAttachParent`))) (`KismetMathLibrary.ComposeRotators` _returnvalue_2 (struct :`Yaw` 270.0)) true false)))