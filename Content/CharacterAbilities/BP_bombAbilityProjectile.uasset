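; Bomb projectile for a character ability that arcs to a destination, then explodes to damage enemies.
; InitBomb builds a three-point spline with a raised midpoint, which Tick follows using a counter scaled by FuseTime.
; When the counter reaches FuseTime, Explode swaps to the explosion flipbook and sphere-traces pawns to damage valid BP_BaseEnemy hits, with debug drawing on.
; A timer set to the flipbook's length then destroys the actor.
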(event `self.ReceiveTick`
  (params (DeltaSeconds :type "Float (single-precision)"))
  (if (`self.initialised`)
    (bind _output_get (set `self.splineTimeCounter` (+ (* (/ DeltaSeconds (`self.fuseTime`)) 10.0) (`self.splineTimeCounter`))))
    (`SceneComponent.K2_SetWorldLocation` (`self.RenderComponent`) (`SplineComponent.GetLocationAtTime` (`self.bombTrajectory`) (/ _output_get (`self.fuseTime`)) "Local" false) false false)
    (if (and (>= (`self.splineTimeCounter`) (`self.fuseTime`)) (not (`self.exploded`)))
      (`self.explode`)
      (`KismetSystemLibrary.K2_SetTimerDelegate` (delegate `DestroyBomb`) (`PaperFlipbookComponent.GetFlipbookLength` (`self.RenderComponent`))))))

(event `DestroyBomb`
  (`self.K2_DestroyActor`))

(fn `explode`
  (bind _returnvalue (`SceneComponent.K2_GetComponentLocation` (`self.RenderComponent`)))
  (`PaperFlipbookComponent.SetLooping` (`self.RenderComponent`) false)
  (`PaperFlipbookComponent.SetFlipbook` (`self.RenderComponent`) "/Game/CharacterAbilities/sprites/Bomb_Explosion.Bomb_Explosion")
  (set `self.exploded` true)
  (bind _outhits (`KismetSystemLibrary.SphereTraceMultiForObjects` :`Start` _returnvalue :`End` _returnvalue :`Radius` (`self.explosionRadius`) :`ObjectTypes` (`|MakeArray` "ObjectTypeQuery3" :!type "EObjectTypeQuery Enum") :`DrawDebugType` "ForDuration" :`DrawTime` 1.0))
  (for _array_element _outhits
    (bind (_bblockinghit _binitialoverlap _time _distance _location _impactpoint _normal _impactnormal _physmat _hitactor) (`GameplayStatics.BreakHitResult` _array_element))
    (if (`/Game/CharacterAbilities/BML_characterAbilityMacros.isValidEnemy` _hitactor)
      (bind _asbp_base_enemy (cast `/Game/Enemies/BP_BaseEnemy` _hitactor))
      (`/Game/Enemies/BP_BaseEnemy.TakeDamage` _asbp_base_enemy (`self.bombDamage`)))))

(fn `initBomb`
  (params (startLocation :type "Vector Structure") (Destination :type "Vector Structure") (fuseTime :type "Float (double-precision)"))
  (set `self.startLocation` startLocation)
  (set `self.bombDestination` Destination)
  (set `self.fuseTime` fuseTime)
  (`SplineComponent.SetSplinePoints` (`self.bombTrajectory`) (`|MakeArray` (`local.startLocation`) (+ (+ (/ (- (`self.bombDestination`) (`local.startLocation`)) 2.0) (`local.startLocation`)) (0.0 0.0 200.0)) (`self.bombDestination`)) "Local" true)
  (set `self.initialised` true))

(fn `UserConstructionScript`
  (`SceneComponent.K2_SetRelativeRotation` (`self.RenderComponent`) (struct :`Yaw` 90.0) false false))