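; Projectile for the paint brush ability that applies a poison, stun or slow effect to enemies it touches.
; A non-looping animation on the render component drives it: each frame change lengthens the collision along its X scale, and the actor destroys itself when playback finishes.
; Collision overlaps with valid enemies switch on BrushEffect and call the matching BP_BaseEnemy function, with only slow taking its settings from variables.
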(event `self.ReceiveBeginPlay`
  (`parent.ReceiveBeginPlay`))

(event `self.ReceiveTick`
  (params (DeltaSeconds :type "Float (single-precision)"))
  (bind _returnvalue (`PaperFlipbookComponent.GetPlaybackPositionInFrames` (`self.RenderComponent`)))
  (`parent.ReceiveTick` DeltaSeconds)
  (if (!= _returnvalue (`self.currentFrame`))
    (set `self.currentFrame` _returnvalue)
    (`SceneComponent.SetWorldScale3D` (`self.collision`) (`KismetMathLibrary.MakeVector` (+ (.x (`SceneComponent.K2_GetComponentScale` (`self.collision`))) 1.0) (.y (`SceneComponent.K2_GetComponentScale` (`self.collision`))) (.z (`SceneComponent.K2_GetComponentScale` (`self.collision`)))))))

(event `self.RenderComponent.OnFinishedPlaying`
  (`self.K2_DestroyActor`))

(event `self.collision.OnComponentBeginOverlap`
  (params (OverlappedComponent :type "PrimitiveComponent Object Reference") (OtherActor :type "Actor Object Reference") (OtherComp :type "PrimitiveComponent Object Reference") (OtherBodyIndex :type Integer) (bFromSweep :type Boolean) (SweepResult :type "HitResult Structure (by ref)"))
  (if (`/Game/CharacterAbilities/GenericClasses/BML_characterAbilityMacros.isValidEnemy` OtherActor)
    (bind _asbp_base_enemy (cast `/Game/Enemies/BP_BaseEnemy` OtherActor))
    (switch `/Game/CharacterAbilities/Enum_brushAbilityBrushTypes` (`self.brushEffect`)
      (:`NewEnumerator0`
        (`/Game/Enemies/BP_BaseEnemy.PoisonEnemy` _asbp_base_enemy 20 3.0 0.5))
      (:`NewEnumerator1`
        (`/Game/Enemies/BP_BaseEnemy.StunEnemy` _asbp_base_enemy 2.0))
      (:`NewEnumerator2`
        (`/Game/Enemies/BP_BaseEnemy.SlowEnemy` _asbp_base_enemy (`self.slowPercentage`) (`self.slowDuration`))))
    (else
      (`KismetSystemLibrary.PrintString` "invalid enemy"))))

(fn `UserConstructionScript`
  (`parent.UserConstructionScript`)
  (`PaperFlipbookComponent.SetLooping` (`self.RenderComponent`) false))