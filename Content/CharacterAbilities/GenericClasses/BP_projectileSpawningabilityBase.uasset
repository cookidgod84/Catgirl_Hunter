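; Base component for projectile-spawning abilities, supplying fire timing and nearest-enemy targeting helpers; it spawns nothing itself.
; IncrementFiringTimer accumulates delta time and returns true when FireRate, used as an interval, is reached, carrying over the remainder.
; Two search functions find the enemy closest to the attach parent, from an actor list or from hit results cast to BP_BaseEnemy.
; Both fall back to the parent's location when no valid enemy exists.
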(fn `findNearestEnemyLocation`
  (params (PotentialEnemies :type "Array of /Game/Enemies/BP_BaseEnemy Object Reference"))
  (returns (nearestEnemyLocation :type "Vector Structure"))
  (locals (nearestEnemyDistance :type "Float (double-precision)" :default 1000000.0) (currentNearestEnemy :type "/Game/Enemies/BP_BaseEnemy Object Reference"))
  (for _array_element PotentialEnemies
    (bind _returnvalue (`KismetMathLibrary.Vector_Distance` (`Actor.K2_GetActorLocation` _array_element) (`self.K2_GetComponentLocation` (`self.GetAttachParent`))))
    (if (< _returnvalue (`local.nearestEnemyDistance`))
      (set `local.nearestEnemyDistance` _returnvalue)
      (set `local.currentNearestEnemy` _array_element)))
  (if (`KismetSystemLibrary.IsValid` (`local.currentNearestEnemy`))
    (return (`Actor.K2_GetActorLocation` (`local.currentNearestEnemy`)))
    (else
      (return (`self.K2_GetComponentLocation` (`self.GetAttachParent`))))))

(fn `findNearestEnemyLocationFromHitResults`
  (params (hitresults :type "Array of HitResult Structure"))
  (returns (nearestEnemyLocation :type "Vector Structure") (nearestEnemy :type "/Game/Enemies/BP_BaseEnemy Object Reference"))
  (locals (nearestEnemyDistance :type "Float (double-precision)" :default 1000000.0) (currentNearestEnemy :type "/Game/Enemies/BP_BaseEnemy Object Reference"))
  (bind _currentnearestenemy (`local.currentNearestEnemy`))
  (for _array_element hitresults
    (bind _asbp_base_enemy (cast `/Game/Enemies/BP_BaseEnemy` (`.HitActor` (`GameplayStatics.BreakHitResult` _array_element))))
    (bind _returnvalue (`KismetMathLibrary.Vector_Distance` (`Actor.K2_GetActorLocation` _asbp_base_enemy) (`self.K2_GetComponentLocation` (`self.GetAttachParent`))))
    (if (< _returnvalue (`local.nearestEnemyDistance`))
      (set `local.nearestEnemyDistance` _returnvalue)
      (set `local.currentNearestEnemy` _asbp_base_enemy)))
  (if (`KismetSystemLibrary.IsValid` (`local.currentNearestEnemy`))
    (return (`Actor.K2_GetActorLocation` _currentnearestenemy) _currentnearestenemy)
    (else
      (return (`self.K2_GetComponentLocation` (`self.GetAttachParent`)) null))))

(fn `Increment Firing Timer`
  (params (deltaSeconds :type "Float (double-precision)"))
  (returns (spawnProjectile :type Boolean))
  (bind _output_get (set `self.fireRateCounter` (+ deltaSeconds (`self.fireRateCounter`))))
  (if (>= _output_get (`self.fireRate`))
    (set `self.fireRateCounter` (- (`self.fireRateCounter`) (`self.fireRate`)))
    (return true)
    (else
      (return false))))