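; Base Blueprint for arcing ability projectiles that builds a curved trajectory when play begins.
; InitSpline clears the Trajectory spline and rebuilds it from StartLocation, a midpoint raised by ArcHeight, and EndLocation, all set in local space.
; Tick only calls the parent, so this graph does not itself move anything along the spline.
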(event `self.ReceiveBeginPlay`
  (`parent.ReceiveBeginPlay`)
  (`self.InitSpline`))

(event `self.ReceiveTick`
  (params (DeltaSeconds :type "Float (single-precision)"))
  (`parent.ReceiveTick` DeltaSeconds))

(fn `InitSpline`
  (bind _trajectory (`self.Trajectory`))
  (`SplineComponent.ClearSplinePoints` _trajectory true)
  (`SplineComponent.SetSplinePoints` _trajectory (`|MakeArray` (`self.StartLocation`) (+ (/ (+ (`self.EndLocation`) (`self.StartLocation`)) 2.0) (`KismetMathLibrary.MakeVector` 0.0 0.0 (`self.ArcHeight`))) (`self.EndLocation`)) "Local" true))

(fn `UserConstructionScript`
  (`parent.UserConstructionScript`))