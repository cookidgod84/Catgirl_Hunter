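; Whip ability Blueprint that automatically fires at enemies near the actor it is attached to.
; Tick advances a firing timer; when it fires, a sphere trace within the max whip range gathers Pawns, ignoring the player character.
; The nearest enemy from those hits is passed, with start and end locations, to a newly spawned whip projectile.
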(event `self.ReceiveTick`
  (params (DeltaSeconds :type "Float (single-precision)"))
  (bind _returnvalue (`self.K2_GetComponentLocation` (`self.GetAttachParent`)))
  (bind _returnvalue_2 (`self.K2_GetComponentLocation` (`self.GetAttachParent`)))
  (`parent.ReceiveTick` DeltaSeconds)
  (bind _spawnprojectile (`self.Increment Firing Timer` DeltaSeconds))
  (if _spawnprojectile
    (bind _outhits (`KismetSystemLibrary.SphereTraceMultiForObjects` _returnvalue _returnvalue (`self.maxwhiprange`) (`|MakeArray` "ObjectTypeQuery3" :!type "EObjectTypeQuery Enum") false (`|MakeArray` (`GameplayStatics.GetPlayerCharacter` 0) :!type "Actor Object Reference")))
    (bind (_nearestenemylocation _nearestenemy) (`self.findNearestEnemyLocationFromHitResults` _outhits))
    (`|SpawnActorFromClass` "/Game/CharacterAbilities/BP_whipAbilityProjectile.BP_whipAbilityProjectile_C" (`KismetMathLibrary.MakeTransform` _returnvalue_2) "Undefined" "MultiplyWithRoot" null _nearestenemylocation _returnvalue_2 _nearestenemy null)))