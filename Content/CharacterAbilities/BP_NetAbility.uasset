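; BP_NetAbility is a character ability component that automatically launches net projectiles from the component it is attached to.
; Each tick it advances a firing timer and, when that returns true, spawns a BP_NetAbilityProjectile at the attach parent's location.
; The projectile receives a net radius, arc height and start point, plus a random landing point between minimum and maximum range around the parent.
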(event `self.ReceiveTick`
  (params (DeltaSeconds :type "Float (single-precision)"))
  (bind _returnvalue (`self.K2_GetComponentLocation` (`self.GetAttachParent`)))
  (`parent.ReceiveTick` DeltaSeconds)
  (bind _spawnprojectile (`self.Increment Firing Timer` DeltaSeconds))
  (if _spawnprojectile
    (`|SpawnActorFromClass` "/Game/CharacterAbilities/BP_NetAbilityProjectile.BP_NetAbilityProjectile_C" (`KismetMathLibrary.Conv_VectorToTransform` (`self.K2_GetComponentLocation` (`self.GetAttachParent`))) "Undefined" "MultiplyWithRoot" null (`self.netRadius`) _returnvalue (`/Game/CharacterAbilities/GenericClasses/BML_characterAbilityMacros.RandomPointInRange` (`self.netMaxRange`) (`self.netMinRange`) _returnvalue) (`self.netArcHeight`) null)))