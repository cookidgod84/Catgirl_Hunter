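; Projectile actor for the clay wire ability that damages enemies its wire touches.
; On BeginPlay it slides the left hand flipbook to a relative offset built from the actor's right vector and travel distance, then destroys itself after the two-second move.
; WireMesh overlaps with BP_BaseEnemy deal damage as a percentage of that enemy's max health, truncated to an integer.
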(event `self.ReceiveBeginPlay`
  (`parent.ReceiveBeginPlay`)
  (`KismetSystemLibrary.MoveComponentTo` (`self.LeftHandFlipbook`) (* (`KismetMathLibrary.GetRightVector` (`self.K2_GetActorRotation`)) (`self.traveldistance`)) (struct) false false 2.0)
  (`self.K2_DestroyActor`))

(event `self.WireMesh.OnComponentBeginOverlap`
  (params (OverlappedComponent :type "PrimitiveComponent Object Reference") (OtherActor :type "Actor Object Reference") (OtherComp :type "PrimitiveComponent Object Reference") (OtherBodyIndex :type Integer) (bFromSweep :type Boolean) (SweepResult :type "HitResult Structure (by ref)"))
  (bind _asbp_base_enemy (cast `/Game/Enemies/BP_BaseEnemy` OtherActor))
  (`/Game/Enemies/BP_BaseEnemy.TakeDamage` _asbp_base_enemy (`KismetMathLibrary.FTrunc` (* (`/Game/Enemies/BP_BaseEnemy.maxhealth` _asbp_base_enemy) (`self.percentagedamage`)))))

(fn `UserConstructionScript`
  (`parent.UserConstructionScript`))