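; Player ability actor for a chisel minion that follows the player and fires projectiles at nearby enemies.
; Tick keeps it on the player and ping-pongs the flipbook chisel along a spline, flipping it at each end.
; A shuffled sphere trace around the player picks a random enemy, retrying on a timer when none is found.
; The attack flipbook's completion launches BP_chiselProjectile at the target, then starts the cooldown timer.
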(event `FindChiselTarget`
  (`self.findNextTarget`)
  (if (`KismetSystemLibrary.IsValid` (`self.targetenemy`))
    (set `self.findingtarget` false)
    (else
      (`KismetSystemLibrary.K2_SetTimerDelegate` (delegate `FindChiselTarget`) 0.5))))

(event `self.ReceiveBeginPlay`
  (`self.FindChiselTarget`))

(event `self.ReceiveTick`
  (params (DeltaSeconds :type "Float (single-precision)"))
  (bind _targetenemy (`self.targetenemy`))
  (`self.moveChisel` DeltaSeconds)
  (if (`KismetSystemLibrary.IsValid` _targetenemy)
    (if (not (`/Game/Enemies/BP_BaseEnemy.isDying` _targetenemy))
      (if (not (`self.isattacking`))
        (`self.attack`))
      (else
        (if (not (`self.findingtarget`)) :!label _label
          (`self.FindChiselTarget`))))
    (else
      (goto _label))))

(event `CanFireAgain`
  (set `self.isattacking` false))

(event `self.Chisel.OnFinishedPlaying`
  (`self.launchChisel`)
  (`PaperFlipbookComponent.SetLooping` (`self.Chisel`) true)
  (`PaperFlipbookComponent.SetPlayRate` (`self.Chisel`) 1.0)
  (`PaperFlipbookComponent.SetFlipbook` (`self.Chisel`) "/Game/CharacterAbilities/assets/chiselsummonassets/Chisel_move.Chisel_move")
  (`PaperFlipbookComponent.Play` (`self.Chisel`))
  (`KismetSystemLibrary.K2_SetTimerDelegate` (delegate `CanFireAgain`) (`self.attackspeed`)))

(fn `attack`
  (bind _chisel (`self.Chisel`))
  (set `self.isattacking` true)
  (`PaperFlipbookComponent.SetLooping` (`self.Chisel`) false)
  (`PaperFlipbookComponent.SetPlayRate` _chisel (/ (`PaperFlipbookComponent.GetFlipbookLength` _chisel) (`self.attackspeed`)))
  (`PaperFlipbookComponent.SetFlipbook` (`self.Chisel`) "/Game/CharacterAbilities/assets/chiselsummonassets/Chisel_attack.Chisel_attack")
  (`KismetSystemLibrary.PrintString` "attackin"))

(fn `findNextTarget`
  (bind _returnvalue (`SceneComponent.K2_GetComponentLocation` (`Actor.RootComponent` (`GameplayStatics.GetPlayerPawn` 0))))
  (bind _outhits (`KismetSystemLibrary.SphereTraceMultiForObjects` :`Start` _returnvalue :`End` _returnvalue :`Radius` (`self.newtargetsearchradius`) :`ObjectTypes` (`|MakeArray` "ObjectTypeQuery3" :!type "EObjectTypeQuery Enum") :`DrawDebugType` "ForDuration" :`DrawTime` 1.0))
  (`KismetArrayLibrary.Array_Shuffle` _outhits)
  (for _array_element _outhits
    (bind _asbp_base_enemy (cast `/Game/Enemies/BP_BaseEnemy` (`.HitActor` (`GameplayStatics.BreakHitResult` _array_element))))
    (set `self.targetenemy` _asbp_base_enemy)
    (break)))

(fn `launchChisel`
  (bind _returnvalue (`SceneComponent.K2_GetComponentLocation` (`self.Chisel`)))
  (`|SpawnActorFromClass` "/Game/CharacterAbilities/BP_chiselProjectile.BP_chiselProjectile_C" (`KismetMathLibrary.Conv_VectorToTransform` _returnvalue) "Undefined" "MultiplyWithRoot" null (`KismetMathLibrary.GetDirectionUnitVector` _returnvalue (`self.K2_GetActorLocation` (`self.targetenemy`))) (`self.projectilemovespeed`) (`self.damage`) null))

(fn `moveChisel`
  (params (DeltaTime :type "Float (double-precision)"))
  (`SceneComponent.K2_SetWorldLocation` (`self.DefaultSceneRoot`) (`self.K2_GetActorLocation` (`GameplayStatics.GetPlayerPawn` 0)) false false)
  (bind _output_get (set `self.positiononspline` (+ (* DeltaTime (`self.movespeed`)) (`self.positiononspline`))))
  (if (or (> _output_get 1.0) (< _output_get 0.0))
    (set `self.positiononspline` (`KismetMathLibrary.FClamp` (`self.positiononspline`)))
    (set `self.movespeed` (* (`self.movespeed`) -1.0))
    (`SceneComponent.K2_AddLocalRotation` (`self.Chisel`) (struct :`Yaw` 180.0) false false))
  (`SceneComponent.K2_SetRelativeLocation` (`self.Chisel`) (`SplineComponent.GetLocationAtTime` (`self.movepath`) (`self.positiononspline`) "Local" false) false false))

(fn `UserConstructionScript`
  (`parent.UserConstructionScript`)
  (`SceneComponent.K2_SetRelativeLocation` (`self.Chisel`) (`SplineComponent.GetLocationAtTime` (`self.movepath`) 0.0 "Local" false) false false)
  (`SceneComponent.K2_SetRelativeRotation` (`self.DefaultSceneRoot`) (struct :`Yaw` 270.0) false false))