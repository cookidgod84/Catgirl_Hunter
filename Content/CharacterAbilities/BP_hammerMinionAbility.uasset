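; Hammer minion ability: a Paper2D flipbook minion, using bear zodiac animations, that hunts and attacks BP_BaseEnemy actors.
; FindNextTarget sphere-traces for pawns around itself, or around the player when it strays too far, and retries on a timer while none is found.
; Tick moves it straight toward the target by setting location directly until TryAttack finds it in range.
; Attack then deals damage on a repeating timer until the enemy dies or leaves range.
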(event `FindHammerTarget`
  (`self.findNextTarget`)
  (if (`KismetSystemLibrary.IsValid` (`self.targetenemy`))
    (set `self.findingtarget` false)
    (`PaperFlipbookComponent.SetFlipbook` (`self.Hammer`) "/Game/CharacterAbilities/assets/hammersummonassets/bearzodiac_walk1.bearzodiac_walk1")
    (else
      (`PaperFlipbookComponent.SetFlipbook` (`self.Hammer`) "/Game/CharacterAbilities/assets/hammersummonassets/bearzodiac_idle1.bearzodiac_idle1")
      (`KismetSystemLibrary.K2_SetTimerDelegate` (delegate `FindHammerTarget`) 0.5))))

(event `self.ReceiveBeginPlay`
  (`PaperFlipbookComponent.SetFlipbook` (`self.Hammer`) "/Game/CharacterAbilities/assets/hammersummonassets/bearzodiac_idle1.bearzodiac_idle1")
  (`self.FindHammerTarget`))

(event `self.ReceiveTick`
  (params (DeltaSeconds :type "Float (single-precision)"))
  (if (and (not (`self.findingtarget`)) (not (`KismetSystemLibrary.IsValid` (`self.targetenemy`))))
    (set `self.findingtarget` true)
    (`self.FindHammerTarget`)
    (`KismetSystemLibrary.PrintString` "logic issue")
    (elif (`KismetSystemLibrary.IsValid` (`self.targetenemy`))
      (`self.tryAttack`)
      (if (not (`self.isattacking`))
        (`self.move` DeltaSeconds))
      (else
        (`self.FindHammerTarget`)
        (`KismetSystemLibrary.PrintString` "bad behavioue")))))

(event `Attack`
  (if (and (`KismetSystemLibrary.IsValid` (`self.targetenemy`)) (< (`KismetMathLibrary.Vector_Distance` (`SceneComponent.K2_GetComponentLocation` (`self.DefaultSceneRoot`)) (`self.K2_GetActorLocation` (`self.targetenemy`))) (`self.attackrange`)))
    (`/Game/Enemies/BP_BaseEnemy.TakeDamage` (`self.targetenemy`) (`self.damage`))
    (if (`/Game/Enemies/BP_BaseEnemy.isDying` (`self.targetenemy`))
      (set `self.isattacking` false)
      (`self.findNextTarget`)
      (else
        (`KismetSystemLibrary.K2_SetTimerDelegate` (delegate `Attack`) (`self.attackspeed`))))
    (else
      (`PaperFlipbookComponent.SetFlipbook` (`self.Hammer`) "/Game/CharacterAbilities/assets/hammersummonassets/bearzodiac_idle1.bearzodiac_idle1")
      (set `self.isattacking` false))))

(fn `findNextTarget`
  (bind _returnvalue (`SceneComponent.K2_GetComponentLocation` (`self.Hammer`)))
  (bind _returnvalue_2 (`self.K2_GetActorLocation` (`GameplayStatics.GetPlayerPawn` 0)))
  (if (> (`KismetMathLibrary.Vector_Distance` (`SceneComponent.K2_GetComponentLocation` (`self.Hammer`)) (`self.K2_GetActorLocation` (`GameplayStatics.GetPlayerPawn` 0))) 1000.0)
    (bind _outhits (`KismetSystemLibrary.SphereTraceMultiForObjects` :`Start` _returnvalue_2 :`End` _returnvalue_2 :`Radius` (`self.newtargetsearchradius`) :`ObjectTypes` (`|MakeArray` "ObjectTypeQuery3" :!type "EObjectTypeQuery Enum") :`DrawDebugType` "ForDuration" :`DrawTime` 1.0))
    (else
      (bind _outhits_2 (`KismetSystemLibrary.SphereTraceMultiForObjects` :`Start` _returnvalue :`End` _returnvalue :`Radius` (`self.newtargetsearchradius`) :`ObjectTypes` (`|MakeArray` "ObjectTypeQuery3" :!type "EObjectTypeQuery Enum") :`DrawDebugType` "ForDuration" :`DrawTime` 1.0))))
  (`KismetArrayLibrary.Array_Shuffle` _outhits)
  (for _array_element _outhits_2
    (bind _asbp_base_enemy (cast `/Game/Enemies/BP_BaseEnemy` (`.HitActor` (`GameplayStatics.BreakHitResult` _array_element))))
    (set `self.targetenemy` _asbp_base_enemy)
    (break)))

(fn `move`
  (params (DeltaTime :type "Float (double-precision)"))
  (bind _returnvalue (`SceneComponent.K2_GetComponentLocation` (`self.DefaultSceneRoot`)))
  (`SceneComponent.K2_SetWorldLocation` (`self.DefaultSceneRoot`) (+ _returnvalue (* (`KismetMathLibrary.GetDirectionUnitVector` _returnvalue (`self.K2_GetActorLocation` (`self.targetenemy`))) DeltaTime (`self.movespeed`))) false false))

(fn `tryAttack`
  (if (and (not (`self.isattacking`)) (< (`KismetMathLibrary.Vector_Distance` (`SceneComponent.K2_GetComponentLocation` (`self.DefaultSceneRoot`)) (`self.K2_GetActorLocation` (`self.targetenemy`))) (`self.attackrange`)))
    (`PaperFlipbookComponent.SetFlipbook` (`self.Hammer`) "/Game/CharacterAbilities/assets/hammersummonassets/bearzodiac_attack1.bearzodiac_attack1")
    (set `self.isattacking` true)
    (`self.Attack`)))

(fn `UserConstructionScript`
  (`parent.UserConstructionScript`)
  (`SceneComponent.K2_SetWorldRotation` (`self.Hammer`) (struct :`Yaw` 90.0) false false)
  (`SceneComponent.K2_AddLocalOffset` (`self.Hammer`) (0.0 0.0 90.0) false false))