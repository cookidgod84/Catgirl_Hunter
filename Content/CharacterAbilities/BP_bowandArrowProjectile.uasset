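; BP_bowandArrowProjectile is the projectile actor for the bow and arrow ability, drawn with a Paper2D flipbook that the construction script scales up.
; Tick sweeps it along its negative up vector at a fixed speed, without a movement component, and BeginPlay sets its lifespan.
; Collider overlaps apply Damage to any BP_BaseEnemy through TakeDamage, with no destroy on hit.
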(event `self.ReceiveBeginPlay`
  (`self.SetLifeSpan` (`self.lifespan`)))

(event `self.ReceiveTick`
  (params (DeltaSeconds :type "Float (single-precision)"))
  (`self.K2_SetActorLocation` (+ (* (`self.GetActorUpVector`) (* DeltaSeconds -200.0)) (`self.K2_GetActorLocation`)) true))

(event `self.collider.OnComponentBeginOverlap`
  (params (OverlappedComponent :type "PrimitiveComponent Object Reference") (OtherActor :type "Actor Object Reference") (OtherComp :type "PrimitiveComponent Object Reference") (OtherBodyIndex :type Integer) (bFromSweep :type Boolean) (SweepResult :type "HitResult Structure (by ref)"))
  (bind _asbp_base_enemy (cast `/Game/Enemies/BP_BaseEnemy` OtherActor))
  (`/Game/Enemies/BP_BaseEnemy.TakeDamage` _asbp_base_enemy (`self.damage`)))

(fn `UserConstructionScript`
  (`SceneComponent.SetWorldScale3D` (`self.PaperFlipbook`) (2.0 2.0 1.0)))