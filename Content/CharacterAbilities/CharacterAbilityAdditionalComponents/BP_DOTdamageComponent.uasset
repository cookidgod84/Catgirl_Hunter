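; Actor component that applies damage over time to the BP_BaseEnemy it is attached to.
; On BeginPlay it deals DamagePerTick to its owner, then re-arms a timer every TimePerTick until the accumulated time reaches TotalDuration.
; It stops silently if the owner is not a BP_BaseEnemy, and the Tick event is empty, leaving leftover tick-based logic disconnected.
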(event `self.ReceiveBeginPlay`
  (`self.DOTDamageTick`))

(event `self.ReceiveTick`
  (params (DeltaSeconds :type "Float (single-precision)")))

(event `DOTDamageTick`
  (bind _asbp_base_enemy (cast `/Game/Enemies/BP_BaseEnemy` (`self.GetOwner`)))
  (`/Game/Enemies/BP_BaseEnemy.TakeDamage` _asbp_base_enemy (`self.damagePerTick`))
  (bind _output_get (set `self.dotDamageTimer` (+ (`self.dotDamageTimer`) (`self.timePerTick`))))
  (if (< _output_get (`self.totalDuration`))
    (`KismetSystemLibrary.K2_SetTimerDelegate` (delegate `DOTDamageTick`) (`self.timePerTick`))))