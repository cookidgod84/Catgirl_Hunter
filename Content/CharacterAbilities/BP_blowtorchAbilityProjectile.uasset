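; Blowtorch ability projectile: a Paper2D flame that sweeps across an arc and burns the enemies it touches.
; Every 0.05 seconds Tick rotates the flipbook one degree and line-traces along the angle, calling BurnEnemy and ignoring enemies already hit.
; Flipbook completion drives start, loop and end states, destroying the actor after the end animation.
; UseBlowtorch is empty, and its sphere-trace burn code never runs.
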(event `self.ReceiveBeginPlay`
  (`parent.ReceiveBeginPlay`)
  (`PaperFlipbookComponent.SetFlipbook` (`self.BlowtorchFlipbook`) "/Game/CharacterAbilities/assets/blowtorchassets/blowtorchflamestart.blowtorchflamestart")
  (`PaperFlipbookComponent.SetLooping` (`self.BlowtorchFlipbook`) false)
  (`SceneComponent.K2_SetRelativeRotation` (`self.BlowtorchFlipbook`) (`KismetMathLibrary.MakeRotator` 90.0 0.0 (+ (`self.angle`) 90.0)) false false))

(event `self.ReceiveTick`
  (params (DeltaSeconds :type "Float (single-precision)"))
  (`parent.ReceiveTick` DeltaSeconds)
  (bind _output_get (set `self.timer` (+ DeltaSeconds (`self.timer`))))
  (if (> _output_get 0.05)
    (set `self.timer` (- (`self.timer`) 0.05))
    (if (and (< (`self.tickcounter`) (`self.sectorsize`)) (!= (`self.blowtorchstate`) 2))
      (`SceneComponent.K2_AddRelativeRotation` (`self.BlowtorchFlipbook`) (struct :`Yaw` 1.0) false false)
      (bind _outhits (`KismetSystemLibrary.LineTraceMultiForObjects` (`self.K2_GetActorLocation`) (`self.getEndPointForTrace`) (`|MakeArray` "ObjectTypeQuery3" :!type "EObjectTypeQuery Enum") false (`self.hitenemies`) "ForOneFrame" true (struct :`R` 1.0 :`A` 1.0) (struct :`G` 1.0 :`A` 1.0) 1.0))
      (for _array_element _outhits
        (bind _asbp_base_enemy (cast `/Game/Enemies/BP_BaseEnemy` (`.HitActor` (`GameplayStatics.BreakHitResult` _array_element))))
        (`/Game/Enemies/BP_BaseEnemy.BurnEnemy` _asbp_base_enemy (`self.burndamage`) (`self.burnduration`))
        (`KismetArrayLibrary.Array_Add` (`self.hitenemies`) _asbp_base_enemy))
      (set `self.tickcounter` (+ (`self.tickcounter`) 1.0))
      (if (== (`self.angle`) 359.0)
        (set `self.angle` 0.0)
        (else
          (set `self.angle` (+ (`self.angle`) 1.0))))
      (else
        ;[1 1 1] blowtorch has finished its sweep
        (set `self.blowtorchstate` 2)
        (`PaperFlipbookComponent.SetFlipbook` (`self.BlowtorchFlipbook`) "/Game/CharacterAbilities/assets/blowtorchassets/blowtorchflameend.blowtorchflameend")
        (`PaperFlipbookComponent.SetLooping` (`self.BlowtorchFlipbook`) false)))))

(event `self.BlowtorchFlipbook.OnFinishedPlaying`
  ;[1 1 1] changing blowtorch state
  (switch `int` (`self.blowtorchstate`)
    (:`0`
      (`PaperFlipbookComponent.SetFlipbook` (`self.BlowtorchFlipbook`) "/Game/CharacterAbilities/assets/blowtorchassets/blowtorchflame1.blowtorchflame1")
      (`PaperFlipbookComponent.SetLooping` (`self.BlowtorchFlipbook`) true)
      (`PaperFlipbookComponent.Play` (`self.BlowtorchFlipbook`))
      (set `self.blowtorchstate` 1))
    (:`2`
      (`self.K2_DestroyActor`))))

(fn `useBlowtorch`)

(fn `UserConstructionScript`
  (`parent.UserConstructionScript`))