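; Clay wire ability component that periodically fires BP_clayWireAbilityProjectile from random points around the component it is attached to.
; Each Tick advances a firing timer through IncrementFiringTimer and spawns a projectile when it returns true, passing in percentage damage and travel distance.
; MakeWireStartLocation builds the spawn transform from randomly signed X/Y offsets around the parent's location, with forward aimed back toward the parent.
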(event `self.ReceiveTick`
  (params (DeltaSeconds :type "Float (single-precision)"))
  (bind _spawnprojectile (`self.Increment Firing Timer` DeltaSeconds))
  (if _spawnprojectile
    (bind _wiretransform (`self.makeWireStartLocation`))
    (`|SpawnActorFromClass` "/Game/CharacterAbilities/BP_clayWireAbilityProjectile.BP_clayWireAbilityProjectile_C" _wiretransform "Undefined" "MultiplyWithRoot" null (`self.wirepercentagedamage`) (`self.wiretraveldistance`) null)))

(fn `makeWireStartLocation`
  (returns (wireTransform :type "Transform Structure"))
  (locals (negators :type "Array of Integer"))
  (bind _returnvalue (+ (`KismetMathLibrary.MakeVector` (+ (`self.minwirespawnrange`) (* (* (`self.maxwirespawnrange`) (`KismetMathLibrary.RandomFloat`)) (`|GetArrayItem` (`local.negators`) (`KismetMathLibrary.Conv_Int64ToInt` (`KismetMathLibrary.RandomInteger64InRange` 0 1))))) (+ (`self.minwirespawnrange`) (* (* (`self.maxwirespawnrange`) (`KismetMathLibrary.RandomFloat`)) (`|GetArrayItem` (`local.negators`) (`KismetMathLibrary.Conv_Int64ToInt` (`KismetMathLibrary.RandomInteger64InRange` 0 1)))))) (`self.K2_GetComponentLocation` (`self.GetAttachParent`))))
  (return (`KismetMathLibrary.MakeTransform` _returnvalue (`KismetMathLibrary.MakeRotationFromAxes` (- (`self.K2_GetComponentLocation` (`self.GetAttachParent`)) _returnvalue) (0.0 0.0 0.0) (0.0 1.0 0.0)))))