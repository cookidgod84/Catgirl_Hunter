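; Paint brush character ability that periodically spawns brush stroke projectiles on the nearest enemy.
; Each time the firing timer elapses on Tick, it gathers all BP_BaseEnemy actors and finds the closest one's location.
; The stroke spawns there at zero height with random yaw and a randomly chosen brush effect type, receiving the ability's slow and stun settings.
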(event `self.ReceiveTick`
  (params (DeltaSeconds :type "Float (single-precision)"))
  (`parent.ReceiveTick` DeltaSeconds)
  (bind _spawnprojectile (`self.Increment Firing Timer` DeltaSeconds))
  (if _spawnprojectile
    (bind _outactors (`GameplayStatics.GetAllActorsOfClass` "/Game/Enemies/BP_BaseEnemy.BP_BaseEnemy_C"))
    (bind _nearestenemylocation (`self.findNearestEnemyLocation` _outactors))
    (bind _transform (`self.Make Brush Stroke Transform` _nearestenemylocation))
    (`|SpawnActorFromClass` "/Game/CharacterAbilities/BP_paintBrushAbilityProjectile.BP_paintBrushAbilityProjectile_C" _transform "Undefined" "MultiplyWithRoot" null (cast `/Game/CharacterAbilities/Enum_brushAbilityBrushTypes` (`KismetMathLibrary.Conv_IntToByte` (`KismetSystemLibrary.MakeLiteralInt` (`KismetMathLibrary.RandomIntegerInRange` 0 (- (enumcount `/Game/CharacterAbilities/Enum_brushAbilityBrushTypes`) 1))))) (`self.slowPercentage`) (`self.slowDuration`) (`self.stunDuration`) null)))

(fn `Make Brush Stroke Transform`
  (params (nearestEnemy :type "Vector Structure"))
  (returns (transform :type "Transform Structure"))
  (return (`KismetMathLibrary.MakeTransform` (`KismetMathLibrary.MakeVector` (.x nearestEnemy) (.y nearestEnemy)) (`KismetMathLibrary.MakeRotator` 0.0 0.0 (`KismetMathLibrary.RandomFloatInRange` 0.0 360.0)))))