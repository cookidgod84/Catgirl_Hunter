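; Bow-and-arrow ability component that automatically fires arrow projectiles toward the nearest enemy.
; Each tick advances a firing timer; when it triggers, all BP_BaseEnemy actors are searched by distance from the attach parent.
; BP_bowandArrowProjectile spawns at the parent, its Z axis pointing away from the target, with a slightly offset fallback point when none is valid.
; Nearest-enemy distance and reference are not reset between searches here.
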(event `self.ReceiveTick`
  (params (DeltaSeconds :type "Float (single-precision)"))
  (bind _spawnprojectile (`self.Increment Firing Timer` DeltaSeconds))
  (if _spawnprojectile
    (bind _outactors (`GameplayStatics.GetAllActorsOfClass` "/Game/Enemies/BP_BaseEnemy.BP_BaseEnemy_C"))
    (bind _nearestenemylocation (`self.getNearestEnemyLocation` _outactors))
    (bind _transform (`self.makeArrowTransform` _nearestenemylocation))
    (`|SpawnActorFromClass` "/Game/CharacterAbilities/BP_bowandArrowProjectile.BP_bowandArrowProjectile_C" _transform "Undefined" "MultiplyWithRoot" null null)))

(fn `getNearestEnemyLocation`
  (params (enemies :type "Array of /Game/Enemies/BP_BaseEnemy Object Reference"))
  (returns (nearestEnemyLocation :type "Vector Structure"))
  (locals (nearestEnemyDistance :type "Float (double-precision)" :default 1000000.0) (currentNearestEnemy :type "/Game/Enemies/BP_BaseEnemy Object Reference"))
  (for _array_element enemies
    (bind _returnvalue (`KismetMathLibrary.Vector_Distance` (`Actor.K2_GetActorLocation` _array_element) (`self.K2_GetComponentLocation` (`self.GetAttachParent`))))
    (if (< _returnvalue (`local.nearestEnemyDistance`))
      (set `local.nearestEnemyDistance` _returnvalue)
      (set `local.currentNearestEnemy` _array_element)
      (`KismetSystemLibrary.LogString` "found nearest enemy")))
  (if (`KismetSystemLibrary.IsValid` (`local.currentNearestEnemy`))
    (return (`Actor.K2_GetActorLocation` (`local.currentNearestEnemy`)))
    (else
      (return (+ (`self.K2_GetComponentLocation` (`self.GetAttachParent`)) (0.0 1.0 0.0))))))

(fn `makeArrowTransform`
  (params (nearestEnemyLocation :type "Vector Structure"))
  (returns (transform :type "Transform Structure"))
  (bind _returnvalue (`self.K2_GetComponentLocation` (`self.GetAttachParent`)))
  (`KismetSystemLibrary.PrintString` (`KismetStringLibrary.Conv_VectorToString` _returnvalue))
  (return (`KismetMathLibrary.MakeTransform` _returnvalue (`KismetMathLibrary.MakeRotFromZ` (`KismetMathLibrary.Normal` (- (`self.K2_GetComponentLocation` (`self.GetAttachParent`)) nearestEnemyLocation))))))