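; Enemy spawn manager that spawns a BP_BaseEnemy roughly once per second.
; Tick accumulates delta time in SpawnPoints, subtracting one whenever it exceeds one, then spawns and prints a debug message.
; The transform comes from DecideSpawnLocation, fed the player's location.
; That function holds a random X/Y offset calculation scaled by SpawnDistance, but the result is left unused.
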(event `self.ReceiveTick`
  (params (DeltaSeconds :type "Float (single-precision)"))
  (bind _output_get (set `self.spawnPoints` (+ DeltaSeconds (`self.spawnPoints`))))
  (if (> _output_get 1.0)
    (set `self.spawnPoints` (- (`self.spawnPoints`) 1.0))
    (`|SpawnActorFromClass` "/Game/Enemies/BP_BaseEnemy.BP_BaseEnemy_C" (`KismetMathLibrary.Conv_VectorToTransform` (`self.DecideSpawnLocation` (`Actor.K2_GetActorLocation` (`GameplayStatics.GetPlayerCharacter` 0)))) "Undefined" "MultiplyWithRoot" null null)
    (`KismetSystemLibrary.PrintString` "spawn")))