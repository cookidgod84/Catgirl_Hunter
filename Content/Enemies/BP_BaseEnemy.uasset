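; Base flipbook enemy with health, movement and timed status effects, ending in a death animation before destruction.
; Tick runs MoveEnemy unless stunned or dying, using MakeStandardMoveLocation (whose player-chasing math is unconnected) or a random panic vector.
; Burn and poison add damage-over-time components and Niagara effects; burn also randomly triggers panic.
; Timers end stun, slow and shove immunity, with slows scaling and later dividing current speed.
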(event `self.ReceiveActorBeginOverlap`
  (params (OtherActor :type "Actor Object Reference")))

(event `self.ReceiveBeginPlay`
  (`self.K2_SetActorRotation` (struct :`Yaw` 90.0))
  (set `self.Health` (`self.maxhealth`)))

(event `self.ReceiveTick`
  (params (DeltaSeconds :type "Float (single-precision)"))
  (if (`self.isDying`)
    _
    (elif (not (`self.isStunned`))
      (`self.moveEnemy` DeltaSeconds))))

(event `CanBeShovedAgain`
  (set `self.canbeshoved` true))

(event `ShoveEnemy`
  (params (ShoveVector :type "Vector Structure"))
  (if (`self.canbeshoved`)
    (`self.K2_SetActorLocation` (+ ShoveVector (`self.K2_GetActorLocation`)))
    (set `self.canbeshoved` false)
    (`KismetSystemLibrary.K2_SetTimerDelegate` (delegate `CanBeShovedAgain`) (`self.shoveimmunityduration`))
    (`KismetSystemLibrary.PrintString` "enemy successfully  shoved")))

(event `BurnEnemy`
  (params (BurnDamage :type Integer :default 1) (BurnDuration :type "Float (double-precision)" :default 5.0))
  ;[1 1 1] Burn
  (`AddComponent|NODE_AddBP_DOTdamageComponent-2` :`damagePerTick` BurnDamage :`totalDuration` BurnDuration :`timePerTick` 0.5)
  (bind _returnvalue (`AddComponent|NODE_AddNiagaraComponent-4`))
  (`NiagaraComponent.SetAsset` _returnvalue "/Game/particleeffects/BurnDebuffEmitter_System.BurnDebuffEmitter_System" true)
  (bind _returnvalue_2 (`KismetSystemLibrary.K2_SetTimerDelegate` (delegate `PanicFromBurn`) 0.5 true))
  (`KismetSystemLibrary.K2_SetTimerDelegate` (delegate `EndBurn`) BurnDuration))

(event `PanicFromBurn`
  ;[1 1 1] Burn
  (if (== (`KismetMathLibrary.RandomInteger` 4) 0)
    (`self.PanicEnemy` 0.5)))

(event `EndBurn`
  ;[1 1 1] Burn
  (`KismetSystemLibrary.K2_ClearAndInvalidateTimerHandle` (stale `BurnEnemy` _returnvalue_2))
  (`ActorComponent.K2_DestroyComponent` (stale `BurnEnemy` _returnvalue)))

(event `PanicEnemy`
  (params (panicDuration :type "Float (double-precision)"))
  ;[1 1 1] Panic
  (set `self.panicMovementVector` (`KismetMathLibrary.RandomUnitVector`))
  (`KismetSystemLibrary.K2_SetTimerDelegate` (delegate `EndPanic`) panicDuration))

(event `SlowEnemy`
  (params (SlowPercentage :type "Float (double-precision)" :default 1.0) (SlowDuration :type "Float (double-precision)"))
  ;[1 1 1] Poison
  (`self.ModifyEnemySpeed` SlowPercentage SlowDuration)
  (bind _returnvalue (`AddComponent|NODE_AddNiagaraComponent-3` :`RelativeTransform` (`KismetMathLibrary.MakeTransform` (0.0 0.0 50.0))))
  (`NiagaraComponent.SetAsset` _returnvalue "/Game/particleeffects/SlowDebuffEmitter_System.SlowDebuffEmitter_System" true)
  (`KismetSystemLibrary.K2_SetTimerDelegate` (delegate `EndSlowEnemy`) SlowDuration))

(event `EndPanic`
  ;[1 1 1] Panic
  (set `self.panicMovementVector` (0.0 0.0 0.0)))

(event `EndSlowEnemy`
  ;[1 1 1] Poison
  (`ActorComponent.K2_DestroyComponent` (stale `SlowEnemy` _returnvalue)))

(event `PoisonEnemy`
  (params (tickDamage :type Integer) (PoisonDuration :type "Float (double-precision)" :default 1.0) (timeBetweenPoisonTicks :type "Float (double-precision)"))
  ;[1 1 1] Poison
  (bind _returnvalue (`AddComponent|NODE_AddBP_DOTdamageComponent-0` :`damagePerTick` tickDamage :`totalDuration` PoisonDuration :`timePerTick` timeBetweenPoisonTicks))
  (bind _returnvalue_2 (`AddComponent|NODE_AddNiagaraComponent-2` :`RelativeTransform` (`KismetMathLibrary.MakeTransform` (0.0 0.0 50.0))))
  (`NiagaraComponent.SetAsset` _returnvalue_2 "/Game/particleeffects/PoisonDebuffEmitter_System.PoisonDebuffEmitter_System" true)
  (`KismetSystemLibrary.K2_SetTimerDelegate` (delegate `EndPoison`) PoisonDuration))

(event `EndPoison`
  ;[1 1 1] Poison
  (`ActorComponent.K2_DestroyComponent` (stale `PoisonEnemy` _returnvalue))
  (`ActorComponent.K2_DestroyComponent` (stale `PoisonEnemy` _returnvalue_2)))

(event `BeginDying`
  ;[1 1 1] Dying
  (set `self.isDying` true)
  (`PaperFlipbookComponent.SetLooping` (`self.RenderComponent`) false)
  (`PaperFlipbookComponent.SetFlipbook` (`self.RenderComponent`) "/Game/Enemies/basic_enemy_sprites/demo_bat_die.demo_bat_die")
  (`KismetSystemLibrary.K2_SetTimerDelegate` (delegate `FinishDying`) (`PaperFlipbookComponent.GetFlipbookLength` (`self.RenderComponent`))))

(event `FinishDying`
  ;[1 1 1] Dying
  (`KismetSystemLibrary.PrintString` "kiling enemy")
  (`self.K2_DestroyActor`))

(event `StunEnemy`
  (params (stunDuration :type "Float (double-precision)"))
  ;[1 1 1] Stun
  (`PaperFlipbookComponent.SetSpriteColor` (`self.RenderComponent`) (struct :`R` 1.0 :`G` 0.899586 :`B` 0.401155 :`A` 1.0))
  (`PaperFlipbookComponent.Stop` (`self.RenderComponent`))
  (set `self.isStunned` true)
  (`KismetSystemLibrary.K2_SetTimerDelegate` (delegate `EndStun`) stunDuration))

(event `ModifyEnemySpeed`
  (params (speedmodifier :type "Float (double-precision)" :default 1.0) (modifierduration :type "Float (double-precision)"))
  ;[1 1 1] speedmodifier
  (set `self.currentMoveSpeed` (* (`self.currentMoveSpeed`) speedmodifier))
  (`KismetSystemLibrary.K2_SetTimerDelegate` (delegate `RevertEnemySpeedTimingEvent`) modifierduration))

(event `EndStun`
  ;[1 1 1] Stun
  (`PaperFlipbookComponent.SetSpriteColor` (`self.RenderComponent`) (struct :`R` 1.0 :`G` 1.0 :`B` 1.0 :`A` 1.0))
  (`PaperFlipbookComponent.Play` (`self.RenderComponent`))
  (set `self.isStunned` false))

(event `RevertEnemySpeedTimingEvent`
  ;[1 1 1] speedmodifier
  (`self.RevertEnemySpeed` (stale `ModifyEnemySpeed` speedmodifier)))

(event `RevertEnemySpeed`
  (params (speedmodifier :type "Float (double-precision)"))
  ;[1 1 1] speedmodifier
  (set `self.currentMoveSpeed` (/ (`self.currentMoveSpeed`) speedmodifier)))

(event `TakeDamage`
  (params (damage :type Integer))
  ;[1 1 1] taking damage
  (if (not (`self.isDying`))
    (set `self.Health` (- (`self.Health`) damage))
    (if (<= (`self.Health`) 0)
      (`self.BeginDying`))))

(fn `moveEnemy`
  (params (DeltaTime :type "Float (double-precision)"))
  (bind _panicmovementvector (`self.panicMovementVector`))
  (if (== _panicmovementvector (0.0 0.0 0.0))
    (switch `/Game/Enemies/EnemyMoveModes` (`self.moveMode`)
      (:`NewEnumerator0`
        (`self.K2_SetActorLocation` (`self.MakeStandardMoveLocation` DeltaTime) true)))
    (else
      (`self.K2_SetActorLocation` (+ (* _panicmovementvector DeltaTime (`self.currentMoveSpeed`)) (`self.K2_GetActorLocation`)) true))))

(fn `UserConstructionScript`)