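; Base enemy projectile actor that flies in a straight line and destroys itself after a set lifespan.
; BeginPlay starts a timer that calls DestroyEnemyProjectile when Lifespan elapses.
; Each Tick, MoveProjectile offsets the location by Direction, Speed and delta time using a swept move, with no movement component in the logic.
; The overlap event is empty, so no hit or damage response is defined here.
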(event `DestroyEnemyProjectile`
  (`self.K2_DestroyActor`))

(event `self.ReceiveBeginPlay`
  (`KismetSystemLibrary.K2_SetTimerDelegate` (delegate `DestroyEnemyProjectile`) (`self.lifespan`)))

(event `self.ReceiveActorBeginOverlap`
  (params (OtherActor :type "Actor Object Reference")))

(event `self.ReceiveTick`
  (params (DeltaSeconds :type "Float (single-precision)"))
  (`self.moveProjectile` DeltaSeconds))

(fn `moveProjectile`
  (params (`Delta Seconds` :type "Float (double-precision)"))
  (`self.K2_SetActorLocation` (+ (`self.K2_GetActorLocation`) (* `Delta Seconds` (`self.direction`) (`self.speed`))) true))

(fn `UserConstructionScript`)